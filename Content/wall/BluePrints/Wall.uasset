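; Wall actor that the player can chisel through to open a hole that casts light beams.
; Tick accumulates time while the player's trigger overlaps the wall's and chiseling is active; once past Quality, a DoOnce runs ChiselFinished.
; That swaps in the holed mesh, clears the pawn's chisel flag and, for each illuminant the Hole finds, spawns a laser from the hole pointing away from that light source.
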(event EventBeginPlay
  ;[1 1 1] 游戏开始
  (Utilities|FlowControl|Sequence
    (:then_0
      (bind _asbp_player (Utilities|Casting|CastTo (Game|Player|GetPlayerPawn 0)))
      (Variables|Default|SetplayerPawn _asbp_player))
    (:then_1
      (bind _outactors (Actor|GetAllActorsOfClass 0))
      (Variables|Default|SetManger 0 0))))

(event Collision|EventActorBeginOverlap
  (params (OtherActor :type Actor%20Object%20Reference)))

(event EventTick
  (params (DeltaSeconds :type Float%20%28single-precision%29))
  (Utilities|FlowControl|Sequence
    (:then_0
      (Variables|Default|SetCan (Class|PrimitiveComponent|IsOverlappingComponent (Variables|Default|GetTrigger) (Variables|Default|GetGettingTrigger (Variables|Default|GetplayerPawn)))))
    (:then_1
      (if (and (Variables|Default|GetCan) (Variables|Default|GetisChisel))
        (Variables|Default|SetTimer (+ (Variables|Default|GetTimer) (Utilities|Time|GetWorldDeltaSeconds)))))
    (:then_2
      (if (> (Variables|Default|GetTimer) (Variables|Default|Getquality))
        (Variables|Default|SetCan false)
        (Utilities|FlowControl|DoOnce false
          (:Completed
            (CallFunction|ChiselFinished)))))))

(fn ConstructionScript)

(fn ChiselFinished
  (bind _hole (Variables|Default|GetHole))
  (bind _returnvalue (Transformation|GetWorldLocation _hole))
  (Utilities|FlowControl|Sequence
    (:then_0
      (Components|StaticMesh|SetStaticMesh (Variables|Default|Getwall) (Variables|Default|GetwallWithHole)))
    (:then_1
      (Variables|Default|SetisChiesl (Variables|Default|GetplayerPawn) false))
    (:then_2
      (bind (_foundilluminant _illuminantslocation) (Default|FoundLight (Variables|Default|GetHole)))
      (if _foundilluminant
        (for _array_element _illuminantslocation
          (bind _returnvalue_2 (Game|SpawnActorfromClass 0 (Math|Transform|MakeTransform _returnvalue "0, 0, 0" "1,1,1") "Undefined" 0 0))
          (CallFunction|SpawnLaser _returnvalue_2 _returnvalue (+ _returnvalue (* (Math|Vector|Normalize (- _returnvalue _array_element)) 5e+03))))))))