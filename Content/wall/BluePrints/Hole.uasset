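; Hole is a component on a Wall actor that detects which illuminant actors have a clear line to it.
; On begin play it caches the Wall's PlayerPawn so its traces can ignore the player.
; FoundLight line-traces from the hole to every actor tagged "illuminant", returning a found flag and the impact locations of traces that hit an illuminant first.
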(event EventBeginPlay
  (bind _aswall (Utilities|Casting|CastToWall (Components|GetOwner)))
  (Variables|Default|Setplay (Variables|/Game/wall/BluePrints/Wall.Wall_C|GetplayerPawn _aswall)))

(event EventTick
  (params (DeltaSeconds :type Float%20%28single-precision%29)))

(fn FoundLight
  (Utilities|Array|Clear (Variables|Default|GetilluminantsLocation))
  (bind _outactors (Actor|GetAllActorswithTag "illuminant"))
  ;[1 1 1] Found Light
  (bind _output_get (Variables|Default|Setilluminants _outactors))
  (for _array_element _output_get
    (bind _outhit (Collision|LineTraceForObjects (Transformation|GetWorldLocation) (Transformation|GetActorLocation _array_element) (Variables|Default|GetNewVar_0) true (Utilities|Array|MakeArray (Variables|Default|Getplay)) "None" true "(R=1.000000,G=0.000000,B=0.000000,A=1.000000)" "(R=0.000000,G=1.000000,B=0.000000,A=1.000000)" 1e+02))
    (if (.bBlockingHit (Collision|BreakHitResult _outhit))
      (if (Actor|ActorHasTag (.HitActor (Collision|BreakHitResult _outhit)) "illuminant")
        (Variables|Default|SetFoundIlluminant (Actor|ActorHasTag (.HitActor (Collision|BreakHitResult _outhit)) "illuminant"))
        (Utilities|Array|Add (Variables|Default|GetilluminantsLocation) (.Location (Collision|BreakHitResult _outhit))))))
  (return (Variables|Default|GetFoundIlluminant) (Variables|Default|GetilluminantsLocation)))