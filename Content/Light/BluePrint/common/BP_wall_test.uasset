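; Test wall actor that loses Hardness when damaged and, once broken, lets light through as a laser.
; On BeginPlay it caches the first BP_mainLight and BP_manager, though the manager goes unused here.
; Tick watches for depleted Hardness, sets HasHoles and spawns a BP_Light once.
; The laser starts at the wall and points horizontally away from the main light, as if continuing its ray.
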(event Custom|spawn_LIght
  (bind _scene (Variables|Default|GetScene))
  (bind _main_light (Variables|Default|Getmain_light))
  (bind _returnvalue (Transformation|GetWorldLocation _scene))
  (bind _returnvalue_2 (Transformation|GetActorLocation _main_light))
  (bind _returnvalue_3 (- _returnvalue _returnvalue_2))
  (bind _returnvalue_4 (Math|Vector|Normalize _returnvalue_3))
  (bind _returnvalue_5 (* _returnvalue_4 1e+02))
  (bind _returnvalue_6 (+ _returnvalue_5 _returnvalue))
  ;[1 1 1] spawn_light
  (bind _returnvalue_7 (Game|SpawnActorfromClass "/Game/Light/BluePrint/common/BP_Light.BP_Light_C" (Transformation|GetWorldTransform _scene) "Undefined" 0 0))
  (Default|SpawnLaser _returnvalue_7 _returnvalue (Math|Vector|MakeVector (.x _returnvalue_6) (.y _returnvalue_6) (.z (Transformation|GetWorldLocation _scene)))))

(event EventBeginPlay
  ;[1 1 1] begin
  (bind _outactors (Actor|GetAllActorsOfClass "/Game/Light/BluePrint/common/BP_mainLight.BP_mainLight_C"))
  (Variables|Default|Setmain_light (Utilities|Array|Get(acopy) _outactors))
  (bind _outactors_2 (Actor|GetAllActorsOfClass "/Game/Light/BluePrint/Game/BP_manager.BP_manager_C"))
  (Variables|Default|Setmanger (Utilities|Array|Get(acopy) _outactors_2)))

(event Collision|EventActorBeginOverlap
  (params (OtherActor :type Actor%20Object%20Reference)))

(event EventTick
  (params (DeltaSeconds :type Float%20%28single-precision%29))
  ;[1 1 1] tcik
  (if (<= (Variables|Default|Gethardness) 0.0)
    (Variables|Default|Sethas_holes true)
    (Utilities|FlowControl|DoOnce false
      (:Completed
        (CallFunction|SpawnLIght)))))

(event Game|Damage|EventAnyDamage
  (params (Damage :type Float%20%28single-precision%29) (DamageType :type Damage%20Type%20Object%20Reference) (InstigatedBy :type Controller%20Object%20Reference) (DamageCauser :type Actor%20Object%20Reference))
  ;[1 1 1] take damage
  (Variables|Default|Sethardness (- (Variables|Default|Gethardness) Damage)))

(fn ConstructionScript)