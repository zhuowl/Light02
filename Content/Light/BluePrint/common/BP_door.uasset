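; Sliding door actor that toggles open and closed through its door event unless locked, playing a sound at each movement.
; A timeline lerps the wooden mesh's location toward the OpenScene component, and reverses to close it.
; Each timeline update calls UpdateLight on the BP_manager found at BeginPlay, keeping lighting in step with the door.
; When the opener is a BP_character_samurai, the door auto-closes after a short delay.
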(event Custom|door_close
  ;[1 1 1] 播放对应的动画
  (Variables|Default|Setopen? false)
  (Audio|PlaySoundatLocation "/Game/Light/sound/Cue/SoundCue_door.SoundCue_door" (Transformation|GetActorLocation))
  (bind _rotation_value (Timeline|door_open_timeLine Reverse)
    (:Update
      (Transformation|SetWorldLocation (Variables|Default|GetSm_door_wood) (Math|Vector|Lerp(Vector) (Variables|Default|GetTemp_location) (Transformation|GetWorldLocation (Variables|Default|Getopen_scene)) _rotation_value) false false)
      (Default|UpdateLight (Variables|Default|GetManger)))
    (:Finished
      (Utilities|FlowControl|Delay 5.0)
      (if (and (Variables|Default|Getopen?) (.bSuccess (Utilities|Casting|CastToBP_character_samurai (stale Custom|door_open actor))))
        (CallFunction|DoorClose)))))

(event Custom|door_open
  (params (actor :type Actor%20Object%20Reference))
  (bind _sm_door_wood (Variables|Default|GetSm_door_wood))
  ;[1 1 1] 播放对应的动画
  (Variables|Default|Setopen? true)
  (Variables|Default|SetTemp_location (Transformation|GetWorldLocation _sm_door_wood))
  (Audio|PlaySoundatLocation "/Game/Light/sound/Cue/SoundCue_door.SoundCue_door" (Transformation|GetActorLocation))
  (bind _rotation_value (Timeline|door_open_timeLine Play)
    (:Update
      (Transformation|SetWorldLocation _sm_door_wood (Math|Vector|Lerp(Vector) (Variables|Default|GetTemp_location) (Transformation|GetWorldLocation (Variables|Default|Getopen_scene)) _rotation_value) false false)
      (Default|UpdateLight (Variables|Default|GetManger)))
    (:Finished
      (Utilities|FlowControl|Delay 5.0)
      (if (and (Variables|Default|Getopen?) (.bSuccess (Utilities|Casting|CastToBP_character_samurai actor)))
        (CallFunction|DoorClose)))))

(event Custom|door
  (params (actor :type Actor%20Object%20Reference))
  ;[1 1 1] door事件
  (if (not (Variables|Default|GetLock?))
    (if (Variables|Default|Getopen?)
      (CallFunction|DoorClose)
      (else
        (CallFunction|DoorOpen actor)))))

(event EventBeginPlay
  (bind _outactors (Actor|GetAllActorsOfClass "/Game/Light/BluePrint/Game/BP_manager.BP_manager_C"))
  (Variables|Default|SetManger (Utilities|Array|Get(acopy) _outactors)))

(event Collision|EventActorBeginOverlap
  (params (OtherActor :type Actor%20Object%20Reference)))

(event EventTick
  (params (DeltaSeconds :type Float%20%28single-precision%29)))

(fn ConstructionScript)