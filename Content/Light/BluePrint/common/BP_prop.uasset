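; BP_prop is a prop that can be picked up and put down by the player character.
; On BeginPlay it caches the player and the BP_manager.
; Pickup saves its height, applies SmallScale and attaches it to the player's GetScene.
; Drop detaches it at PutScene's X/Y and saved height, restores scale and adds a yaw offset to PutScene's rotation; both actions call the manager's UpdateLight.
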(event EventBeginPlay
  (bind _asbp_character_player (Utilities|Casting|CastToBP_character_player (Game|GetPlayerCharacter 0)))
  (Variables|Default|Setplayer _asbp_character_player)
  (bind _outactors (Actor|GetAllActorsOfClass "/Game/Light/BluePrint/Game/BP_manager.BP_manager_C"))
  (Variables|Default|Setmanger (Utilities|Array|Get(acopy) _outactors)))

(event Collision|EventActorBeginOverlap
  (params (OtherActor :type Actor%20Object%20Reference)))

(event EventTick
  (params (DeltaSeconds :type Float%20%28single-precision%29)))

(fn ConstructionScript)

(fn FUCbeGot
  (bind _player (Variables|Default|Getplayer))
  (bind _get_scene (Variables|/Game/Light/BluePrint/character/BP_character_player.BP_character_player_C|GetGet_scene _player))
  (Variables|Default|SetLocation_z (.z (Transformation|GetActorLocation)))
  (Transformation|SetActorTransform (Math|Transform|MakeTransform (Transformation|GetWorldLocation _get_scene) "0, 0, 0" (Variables|Default|GetSmall_scale)))
  (Transformation|AttachComponentToComponent _get_scene "None" "SnapToTarget" "KeepRelative" "KeepWorld" true)
  (Default|UpdateLight (Variables|Default|Getmanger)))

(fn FUCbeDrop
  (bind _player (Variables|Default|Getplayer))
  (bind _put_scene (Variables|/Game/Light/BluePrint/character/BP_character_player.BP_character_player_C|Getput_scene _player))
  (bind _returnvalue (Transformation|GetWorldRotation _put_scene))
  (bind _returnvalue_2 (Transformation|GetWorldLocation _put_scene))
  ;[1 1 1] 道具被放下
  (Transformation|DetachFromActor "KeepRelative" "KeepRelative" "KeepRelative")
  (Transformation|SetActorTransform (Math|Transform|MakeTransform (Math|Vector|MakeVector (.x _returnvalue_2) (.y _returnvalue_2) (Variables|Default|GetLocation_z)) (Math|Rotator|MakeRotator (.roll _returnvalue) (.pitch _returnvalue) (+ (.yaw _returnvalue) 9e+01)) (Variables|Default|Getback_scale)))
  (Default|UpdateLight (Variables|Default|Getmanger)))