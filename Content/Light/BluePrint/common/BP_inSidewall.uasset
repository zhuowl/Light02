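; Interior side wall Blueprint that procedurally lays out a row of wall segments with one door slot.
; The construction script spawns Count child actors along local X, spaced by WallLength.
; The segment at DoorCount is stretched in X by Bigger + 1, and later segments shift to make room.
; DoorCount is clamped to Count, where no segment is stretched; the event graph is empty.
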(event EventBeginPlay)

(event Collision|EventActorBeginOverlap
  (params (OtherActor :type Actor%20Object%20Reference)))

(event EventTick
  (params (DeltaSeconds :type Float%20%28single-precision%29)))

(fn ConstructionScript
  (bind _wall_length (Variables|Default|Getwall_length))
  (Variables|Default|Setdoor_count (Math|Integer|Clamp(Integer) (Variables|Default|Getdoor_count) 0 (Variables|Default|Getcount)))
  (for _index (range 0 (- (Variables|Default|Getcount) 1))
    (if (== _index (Variables|Default|Getdoor_count))
      (AddComponent|AddChildActorComponent false (Math|Transform|MakeTransform (Math|Vector|MakeVector (* _index _wall_length) 0.0 0.0) "0, 0, 0" (Math|Vector|MakeVector (+ (Variables|Default|Getbigger) 1.0) 1.0 1.0)))
      (else
        (if (> _index (Variables|Default|Getdoor_count))
          (Variables|Default|Setx_value (+ (* _index _wall_length) (* _wall_length (Variables|Default|Getbigger))))
          (else
            (Variables|Default|Setx_value (* _index _wall_length))))
        (AddComponent|AddChildActorComponent false (Math|Transform|MakeTransform (Math|Vector|MakeVector (Variables|Default|Getx_value) 0.0 0.0) "0, 0, 0" "1,1,1"))))))