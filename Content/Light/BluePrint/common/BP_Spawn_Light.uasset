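; Laser emitter Blueprint that fires a beam which bounces off mirror surfaces.
; SpawnLaser line-traces toward a target, stores the ray endpoints, and draws a particle beam up to the first hit.
; Hits on the PM_mirror physical material call FUC_reflect, which recursively traces mirrored rays with no depth limit, adding a beam per segment.
; Update_Laser_List destroys all tracked beams and respawns the laser from the stored endpoints.
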(event Custom|Update_Laser_List
  (bind _incidentlightlist (Variables|Default|GetIncidentLightList))
  ;[1 1 1] 更新光线
  ;;[1 1 1] 遍历光的粒子特效的数组，销毁粒子特效
  (for _array_element _incidentlightlist
    (Components|DestroyComponent _array_element))
  ;;[1 1 1] 清空数组
  (Utilities|Array|Clear _incidentlightlist)
  ;;[1 1 1] 生成光线
  (CallFunction|SpawnLaser (Variables|Default|Getstart) (Variables|Default|GetTempEnd)))

(event Custom|SpawnLaser
  (params (Start :type Vector) (End :type Vector))
  (bind _returnvalue (- End Start))
  (bind _returnvalue_2 (Math|Vector|Normalize _returnvalue))
  (bind _returnvalue_3 (* _returnvalue_2 5e+04))
  (bind _returnvalue_4 (+ Start _returnvalue_3))
  ;[1 1 1] 发出射线
  (Variables|Default|Setstart Start)
  (Variables|Default|SetTempEnd _returnvalue_4)
  (Variables|Default|Setend _returnvalue_4)
  (bind (_outhit _returnvalue_5) (Collision|LineTraceByChannel (Variables|Default|Getstart) (Variables|Default|Getend) "TraceTypeQuery1" true 0 "Persistent"))
  (bind _returnvalue_6 (Effects|SpawnEmitteratLocation "/Game/Light/particle/Laser_Partical.Laser_Partical" (Variables|Default|Getstart)))
  (Utilities|Array|Add (Variables|Default|GetIncidentLightList) _returnvalue_6)
  (if _returnvalue_5
    (Variables|Default|Setend (.Location (Collision|BreakHitResult _outhit)))
    (CallFunction|FUCCreatBeam (Variables|Default|Getstart) (Variables|Default|Getend) _returnvalue_6)
    (if (== (.PhysMat (Collision|BreakHitResult _outhit)) "/Game/Light/Material/Furnishings/PM_mirror.PM_mirror")
      (CallFunction|FUCReflect (Variables|Default|Getstart) (Variables|Default|Getend) _outhit))
    (else
      (CallFunction|FUCCreatBeam (Variables|Default|Getstart) (Variables|Default|Getend) _returnvalue_6))))

(event EventBeginPlay)

(event Collision|EventActorBeginOverlap
  (params (OtherActor :type Actor%20Object%20Reference)))

(event EventTick
  (params (DeltaSeconds :type Float%20%28single-precision%29)))

(fn ConstructionScript)

(fn FUCCreatBeam
  (params (StartLocation :type Vector) (EndLocation :type Vector) (light :type Particle%20System%20Component%20Object%20Reference))
  (Class|ParticleSystemComponent|SetBeamSourcePoint light 0 StartLocation)
  (Class|ParticleSystemComponent|SetBeamEndPoint light 0 EndLocation))

(fn FUCReflect
  (params (Start :type Vector) (End :type Vector) (hit :type Hit%20Result%20Structure))
  (bind (_bblockinghit _binitialoverlap _time _distance _location _impactpoint _normal _impactnormal) (Collision|BreakHitResult hit))
  (LocalVariables|Setreflect_start _impactpoint)
  (LocalVariables|Setreflect_end (+ _impactpoint (* (Math|Vector|Normalize (Math|Vector|MirrorVectorbyNormal (- End Start) _impactnormal)) 5e+03)))
  (bind (_outhit _returnvalue) (Collision|LineTraceByChannel (LocalVariables|Getreflect_start) (LocalVariables|Getreflect_end) "TraceTypeQuery1" true 0 "None"))
  (bind _returnvalue_2 (Effects|SpawnEmitteratLocation "/Game/Light/particle/Laser_Partical.Laser_Partical" (LocalVariables|Getreflect_start)))
  (Utilities|Array|Add (Variables|Default|GetIncidentLightList) _returnvalue_2)
  (if _returnvalue
    (LocalVariables|Setreflect_end (.ImpactPoint (Collision|BreakHitResult _outhit)))
    (CallFunction|FUCCreatBeam (LocalVariables|Getreflect_start) (LocalVariables|Getreflect_end) _returnvalue_2)
    (if (== (.PhysMat (Collision|BreakHitResult _outhit)) "/Game/Light/Material/Furnishings/PM_mirror.PM_mirror")
      (CallFunction|FUCReflect (LocalVariables|Getreflect_start) (LocalVariables|Getreflect_end) _outhit))
    (else
      (CallFunction|FUCCreatBeam (LocalVariables|Getreflect_start) (LocalVariables|Getreflect_end) _returnvalue_2))))