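; BP_Light is a laser light that bounces through mirrors, portals and loupes and brightens lanterns it hits.
; SpawnLaser starts a recursive line-trace chain, with FUC_after_trace spawning a beam emitter per segment and branching on the hit.
; Mirror physical material reflects, Portal tag relays through the paired portal, and Loupe tag bends toward the lens focal point.
; Update_Laser_List destroys the stored emitters and fires the laser again.
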(event Custom|Update_Laser_List
  (bind _incidentlightlist (Variables|Default|GetIncidentLightList))
  ;[1 1 1] 更新光线
  ;;[1 1 1] 遍历光的粒子特效的数组，销毁粒子特效
  (for _array_element _incidentlightlist
    (Components|DestroyComponent _array_element))
  ;;[1 1 1] 清空数组
  (Utilities|Array|Clear _incidentlightlist)
  ;;[1 1 1] 生成光线
  (CallFunction|SpawnLaser (Variables|Default|Getstart) (Variables|Default|GetTempEnd)))

(event Custom|SpawnLaser
  (params (Start :type Vector) (End :type Vector))
  (bind _returnvalue (- End Start))
  (bind _returnvalue_2 (Math|Vector|Normalize _returnvalue))
  (bind _returnvalue_3 (* _returnvalue_2 5e+04))
  (bind _returnvalue_4 (+ Start _returnvalue_3))
  ;[1 1 1] 发出射线
  (Variables|Default|Setstart Start)
  (Variables|Default|SetTempEnd _returnvalue_4)
  (Variables|Default|Setend _returnvalue_4)
  (bind (_outhit _returnvalue_5) (Collision|LineTraceByChannel (Variables|Default|Getstart) (Variables|Default|Getend) "TraceTypeQuery1" true 0 "Persistent"))
  (CallFunction|FUCAfterTrace _outhit (Variables|Default|Getstart) (Variables|Default|Getend) _returnvalue_5))

(event EventBeginPlay
  (bind _outactors (Actor|GetAllActorsOfClass "/Game/Light/BluePrint/Game/BP_manager.BP_manager_C"))
  (Variables|Default|SetManger (Utilities|Array|Get(acopy) _outactors)))

(event Collision|EventActorBeginOverlap
  (params (OtherActor :type Actor%20Object%20Reference)))

(event EventTick
  (params (DeltaSeconds :type Float%20%28single-precision%29)))

(fn ConstructionScript)

(fn FUCCreatBeam
  (params (StartLocation :type Vector) (EndLocation :type Vector) (light :type Particle%20System%20Component%20Object%20Reference))
  (Class|ParticleSystemComponent|SetBeamSourcePoint light 0 StartLocation)
  (Class|ParticleSystemComponent|SetBeamEndPoint light 0 EndLocation))

(fn FUCReflect
  (params (Start :type Vector) (End :type Vector) (hit :type Hit%20Result%20Structure))
  (bind (_bblockinghit _binitialoverlap _time _distance _location _impactpoint _normal _impactnormal) (Collision|BreakHitResult hit))
  ;[1 1 1] 反射
  (LocalVariables|Setreflect_start _impactpoint)
  (LocalVariables|Setreflect_end (+ _impactpoint (* (Math|Vector|Normalize (Math|Vector|MirrorVectorbyNormal (- End Start) _impactnormal)) 5e+03)))
  (bind (_outhit _returnvalue) (Collision|LineTraceByChannel (LocalVariables|Getreflect_start) (LocalVariables|Getreflect_end) "TraceTypeQuery1" true 0 "None"))
  (CallFunction|FUCAfterTrace _outhit (LocalVariables|Getreflect_start) (LocalVariables|Getreflect_end) _returnvalue))

(fn FUCTransfer
  (params (hit_actor :type Actor%20Object%20Reference) (start :type Vector) (Hit_location :type Vector))
  (bind _asbp_portal (Utilities|Casting|CastToBP_portal hit_actor))
  (LocalVariables|Sethit_in_direction (Math|Vector|RotateVector (- Hit_location start) (Math|Rotator|CombineRotators (Transformation|GetActorRotation (Variables|/Game/Light/BluePrint/common/BP_portal.BP_portal_C|Getpair_portal_out _asbp_portal)) (Transformation|GetActorRotation _asbp_portal))))
  (LocalVariables|Settransfer_out_location (+ (Transformation|GetActorLocation (Variables|/Game/Light/BluePrint/common/BP_portal.BP_portal_C|Getpair_portal_out _asbp_portal)) (- Hit_location (Transformation|GetActorLocation _asbp_portal))))
  (LocalVariables|Setend_location (+ (LocalVariables|Gettransfer_out_location) (* (LocalVariables|Gethit_in_direction) 5e+03)))
  (bind (_outhit _returnvalue) (Collision|LineTraceByChannel (LocalVariables|Gettransfer_out_location) (LocalVariables|Getend_location) "TraceTypeQuery1" true 0 "ForDuration" true "(R=1.000000,G=0.000000,B=0.000000,A=1.000000)" "(R=0.000000,G=1.000000,B=0.000000,A=1.000000)" 1e+01))
  (CallFunction|FUCAfterTrace _outhit (LocalVariables|Gettransfer_out_location) (LocalVariables|Getend_location) _returnvalue))

(fn FUCAfterTrace
  (params (Hit :type Hit%20Result%20Structure%20%28by%20ref%29) (Start :type Vector) (End :type Vector) (Condition :type Boolean))
  (bind (_bblockinghit _binitialoverlap _time _distance _location _impactpoint _normal _impactnormal _physmat _hitactor _hitcomponent) (Collision|BreakHitResult Hit))
  ;[1 1 1] 发出检测射线后
  (LocalVariables|Settemp_start Start)
  (LocalVariables|Settemp_end End)
  (bind _returnvalue (Effects|SpawnEmitteratLocation "/Game/Light/particle/Laser_Partical.Laser_Partical" (LocalVariables|Gettemp_start)))
  (Utilities|Array|Add (Variables|Default|GetIncidentLightList) _returnvalue)
  (if Condition
    (LocalVariables|Settemp_end _location)
    (CallFunction|FUCCreatBeam (LocalVariables|Gettemp_start) (LocalVariables|Gettemp_end) _returnvalue)
    (if (== _physmat "/Game/Light/Materials/Furnishings/PM_mirror.PM_mirror")
      (CallFunction|FUCReflect (LocalVariables|Gettemp_start) (LocalVariables|Gettemp_end) Hit)
      (elif (Components|ComponentHasTag _hitcomponent "Portal")
        (CallFunction|FUCTransfer _hitactor (LocalVariables|Gettemp_start) (LocalVariables|Gettemp_end)) ; 反射
        (elif (Components|ComponentHasTag _hitcomponent "Loupe")
          (bind _asbp_loupe (Utilities|Casting|CastToBP_loupe _hitactor))
          (CallFunction|FUCRefract (LocalVariables|Gettemp_start) (LocalVariables|Gettemp_end) _asbp_loupe) ; 折射
          (elif (Actor|ActorHasTag _hitactor "Lantern")
            (bind _asbp_lantern (Utilities|Casting|CastToBP_lantern _hitactor))
            (Default|ToBright _asbp_lantern) ; 点亮
          ))))
    (else
      (CallFunction|FUCCreatBeam (LocalVariables|Gettemp_start) (LocalVariables|Gettemp_end) _returnvalue))))

(fn FUCRefract
  (params (Start :type Vector) (End :type Vector) (loupe :type BP%20Loupe%20Object%20Reference))
  (bind _arrow (Variables|/Game/Light/BluePrint/common/BP_loupe.BP_loupe_C|GetArrow loupe))
  (bind _f_length (Variables|/Game/Light/BluePrint/common/BP_loupe.BP_loupe_C|GetF_length loupe))
  (bind _returnvalue (Math|Vector|GetForwardVector _arrow))
  (bind _returnvalue_2 (Transformation|GetWorldLocation _arrow))
  (bind _returnvalue_3 (* _returnvalue _f_length))
  (LocalVariables|Settemp_start End)
  (LocalVariables|Setin_direction (Math|Vector|Normalize (- End Start)))
  (if (> (Math|Vector|DotProduct _returnvalue (LocalVariables|Getin_direction)) 0.0)
    (LocalVariables|SetF_location (+ _returnvalue_3 _returnvalue_2))
    (LocalVariables|Settemp_end (+ (* (Math|Vector|Normalize (- (LocalVariables|GetF_location) (LocalVariables|Gettemp_start))) 5e+03) (LocalVariables|Gettemp_start)) :!label _label)
    (bind (_outhit _returnvalue_4) (Collision|LineTraceByChannel (LocalVariables|Gettemp_start) (LocalVariables|Gettemp_end) "TraceTypeQuery1" true (Utilities|Array|MakeArray loupe) "ForDuration"))
    (CallFunction|FUCAfterTrace _outhit (LocalVariables|Gettemp_start) (LocalVariables|Gettemp_end) _returnvalue_4)
    (elif (< (Math|Vector|DotProduct _returnvalue (LocalVariables|Getin_direction)) 0.0)
      (LocalVariables|SetF_location (+ (* _returnvalue_3 -1.0) _returnvalue_2))
      (goto _label))))