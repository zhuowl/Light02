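; BP_loupe is a rotatable loupe actor that works with a lighting system managed through its Manger reference.
; Its rotate_loupe event adds the given value as relative yaw to both LoupeMesh and Mesh, then calls UpdateLight on Manger.
; BeginPlay, overlap and Tick are disabled stubs, and the construction script only calls its parent.
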(event Custom|rotate_loupe
  (params (rotate_value :type Float%20%28single-precision%29))
  (Transformation|AddRelativeRotation (Variables|Default|GetLoupe_mesh) (Math|Rotator|MakeRotator 0.0 0.0 rotate_value) false false)
  (Default|UpdateLight (Variables|Default|Getmanger)))

(event EventBeginPlay
  (|CallParentFunction) ; This node is disabled and will not be called.\nDrag off pins to build functionality.
)

(event Collision|EventActorBeginOverlap
  (params (OtherActor :type Actor%20Object%20Reference))
  (|CallParentFunction OtherActor) ; This node is disabled and will not be called.\nDrag off pins to build functionality.
)

(event EventTick
  (params (DeltaSeconds :type Float%20%28single-precision%29))
  (|CallParentFunction DeltaSeconds) ; This node is disabled and will not be called.\nDrag off pins to build functionality.
)

(fn ConstructionScript
  (|CallParentFunction))