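; BP_door is a room door Blueprint that toggles a wooden door mesh between closed and open by sliding it.
; The door event uses a FlipFlop to alternate between open and close.
; Opening caches the mesh's world location, then a timeline lerps it toward the OpenScene component's location.
; Closing reverses the same timeline; despite the track name RotationValue, only location changes.
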(event Custom|door_close
  (bind _rotation_value (Timeline|door_open_timeLine Reverse)
    (:Update
      (Transformation|SetWorldLocation (Variables|Default|GetSm_door_wood) (Math|Vector|Lerp(Vector) (Variables|Default|GetTemp_location) (Transformation|GetWorldLocation (Variables|Default|Getopen_scene)) _rotation_value) false false))))

(event Custom|door_open
  (bind _sm_door_wood (Variables|Default|GetSm_door_wood))
  (Variables|Default|SetTemp_location (Transformation|GetWorldLocation _sm_door_wood))
  (bind _rotation_value (Timeline|door_open_timeLine PlayFromStart)
    (:Update
      (Transformation|SetWorldLocation _sm_door_wood (Math|Vector|Lerp(Vector) (Variables|Default|GetTemp_location) (Transformation|GetWorldLocation (Variables|Default|Getopen_scene)) _rotation_value) false false))))

(event Custom|door
  (Utilities|FlowControl|FlipFlop
    (:A
      (CallFunction|DoorOpen))
    (:B
      (CallFunction|DoorClose))))

(event EventBeginPlay)

(event Collision|EventActorBeginOverlap
  (params (OtherActor :type Actor%20Object%20Reference)))

(event EventTick
  (params (DeltaSeconds :type Float%20%28single-precision%29)))

(fn ConstructionScript)