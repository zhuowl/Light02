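; Procedural room Blueprint that builds a rectangular, modular room from X/Y wall counts in its Construction Script.
; It computes four corner transforms and adds corner meshes, then places wall child actors along each side.
; Wall loops leave gaps for the door and partition junctions according to index and axis settings.
; Functions for doors and an inside partition exist, but their Construction Script calls are disconnected.
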(event EventBeginPlay)

(event Collision|EventActorBeginOverlap
  (params (OtherActor :type Actor%20Object%20Reference)))

(event EventTick
  (params (DeltaSeconds :type Float%20%28single-precision%29)))

(fn ConstructionScript
  (CallFunction|FUCSetConnerWall)
  (CallFunction|FUCSetWall))

(fn FUCSetConTransform
  (bind _wall_con_length (Variables|Conner|Getwall_con_length))
  (bind _start_position (Variables|Default|Getstart_Position))
  (bind _y_wall_count (Variables|Wall|GetY_wall_count))
  (bind _x_wall_count (Variables|Wall|GetX_wall_count))
  (bind _wall_length (Variables|Wall|Getwall_length))
  (bind _wall_length_2 (Variables|Wall|Getwall_length))
  (bind _start_position_2 (Variables|Default|Getstart_Position))
  (bind _wall_con_length_2 (Variables|Conner|Getwall_con_length))
  (bind _wall_con_length_3 (Variables|Conner|Getwall_con_length))
  (bind _returnvalue (* _x_wall_count _wall_length_2))
  (bind _returnvalue_2 (* _y_wall_count _wall_length))
  (bind (_x _y _z) (Math|Vector|BreakVector _start_position_2))
  (bind (_x_2 _y_2 _z_2) (Math|Vector|BreakVector _start_position))
  (bind _returnvalue_3 (+ _returnvalue _wall_con_length_3 _wall_con_length_3 _x))
  (bind _returnvalue_4 (+ _returnvalue_2 _wall_con_length _y_2))
  ;[1 1 1] set conner  location
  (Variables|Conner|Setcon_leftTop_Location (Math|Vector|MakeVector (+ _x _wall_con_length_2) _y _z))
  (Variables|conner|Setcon_rightTop_Location (Math|Vector|MakeVector _returnvalue_3 (+ _y _wall_con_length_2) 0.0))
  (Variables|Conner|Setcon_leftButtom_Location (Math|Vector|MakeVector _x_2 _returnvalue_4 _z_2))
  (Variables|Conner|Setcon_rightButtom_Location (Math|Vector|MakeVector (- _returnvalue_3 _wall_con_length_3) (+ _returnvalue_4 (Variables|Conner|Getwall_con_length)) _z_2))
  ;[1 1 1] set conner rotation
  (Variables|Conner|Setcon_leftTop_rotation "0, 0, 0")
  (Variables|Conner|Setcon_rightTop_rotation "0,90.000000, 0")
  (Variables|Conner|Setcon_leftButtom_rotation "0,-90.000000, 0")
  (Variables|Conner|Setcon_rightButtom_rotation "0,-180.000000, 0"))

(fn FUCSetConnerWall
  ;[1 1 1] 生成 四个墙角
  (CallFunction|FUCSetConTransform)
  (AddComponent|AddStaticMeshComponent false (Math|Transform|MakeTransform (Variables|Conner|Getcon_leftTop_Location) (Variables|Conner|Getcon_leftTop_rotation)))
  (AddComponent|AddStaticMeshComponent false (Math|Transform|MakeTransform (Variables|conner|Getcon_rightTop_Location) (Variables|Conner|Getcon_rightTop_rotation)))
  (AddComponent|AddStaticMeshComponent false (Math|Transform|MakeTransform (Variables|Conner|Getcon_leftButtom_Location) (Variables|Conner|Getcon_leftButtom_rotation)))
  (AddComponent|AddStaticMeshComponent false (Math|Transform|MakeTransform (Variables|Conner|Getcon_rightButtom_Location) (Variables|Conner|Getcon_rightButtom_rotation))))

(fn FUCSetWall
  (bind _start_position (Variables|Default|Getstart_Position))
  (bind _start_position_2 (Variables|Default|Getstart_Position))
  ;[1 1 1] set X wall  生成X方向的可互动墙体
  (for _index (range 0 (- (Variables|Wall|GetX_wall_count) 1))
    (if (Variables|wall_inside|Gethas_Inside_Wall?)
      (if (== (Variables|wall_inside|Getwall__inside_con_count) _index)
        (if (Variables|wall_inside|GetinsideWall_is_inY?)
          (if (Variables|Door|Getdoor_is_inY?) :!label _label
            (AddComponent|AddChildActorComponent false (Math|Transform|MakeTransform (Math|Vector|MakeVector (+ (.x _start_position) (Variables|Conner|Getwall_con_length) (* _index (Variables|Wall|Getwall_length))) (+ (.z _start_position) (Variables|Conner|Getwall_con_width)) (.z _start_position)) "0, 0, 0" "1,1,1") :!label _label_2)
            (elif (== (Variables|Door|Getdoor_in_count) _index)
              _
              (else
                (goto _label_2))))
          (AddComponent|AddChildActorComponent false (Math|Transform|MakeTransform (Math|Vector|MakeVector (+ (.x _start_position) (Variables|Conner|Getwall_con_length) (* _index (Variables|Wall|Getwall_length))) (+ (.y _start_position) (* (Variables|Wall|GetY_wall_count) (Variables|Wall|Getwall_length)) (Variables|Conner|Getwall_con_length) (Variables|Conner|Getwall_con_length)) (.z _start_position)) "0, 0, 0" "1,1,1")))
        (else
          (goto _label)))
      (else
        (goto _label))))
  ;[1 1 1] set Y wall  生成Y方向可互动墙体
  (for _index_2 (range 0 (- (Variables|Wall|GetY_wall_count) 1))
    (if (Variables|wall_inside|Gethas_Inside_Wall?)
      (if (== (Variables|wall_inside|Getwall__inside_con_count) _index_2)
        (if (not (Variables|wall_inside|GetinsideWall_is_inY?))
          (if (Variables|Door|Getdoor_is_inY?) :!label _label_3
            (if (== (Variables|Door|Getdoor_in_count) _index_2)
              _
              (else
                (AddComponent|AddChildActorComponent false (Math|Transform|MakeTransform (Math|Vector|MakeVector (.x _start_position_2) (+ (.y _start_position_2) (* _index_2 (Variables|Wall|Getwall_length)) (Variables|Conner|Getwall_con_length)) (.z _start_position_2)) "0,90.000000, 0" "1,1,1") :!label _label_4)))
            (else
              (goto _label_4)))
          (AddComponent|AddChildActorComponent false (Math|Transform|MakeTransform (Math|Vector|MakeVector (+ (.x _start_position_2) (* (Variables|Wall|GetX_wall_count) (Variables|Wall|Getwall_length)) (Variables|Conner|Getwall_con_length) (Variables|Conner|Getwall_con_length) (* (Variables|Conner|Getwall_con_width) -1.0)) (+ (.y _start_position_2) (* _index_2 (Variables|Wall|Getwall_length)) (Variables|Conner|Getwall_con_length)) (.z _start_position_2)) "0,90.000000, 0" "1,1,1")))
        (else
          (goto _label_3)))
      (else
        (goto _label_3)))))

(fn FUCSetDoor
  (params (Inside_door :type Boolean))
  (bind _wall_con_width (Variables|Conner|Getwall_con_width))
  (if Inside_door
    ;[1 1 1] 放置内门
    (if (Variables|wall_inside|GetinsideWall_is_inY?)
      (Variables|wall_inside|SetinsideDoor_count (Math|Integer|Clamp(Integer) (Variables|wall_inside|GetinsideDoor_count) 0 (- (Variables|Wall|GetX_wall_count) 1)))
      (AddComponent|AddChildActorComponent false (Math|Transform|MakeTransform (Math|Vector|MakeVector (+ (Variables|Conner|Getwall_con_length) (* (Variables|wall_inside|GetinsideDoor_count) (Variables|Wall|Getwall_length))) (+ (* (Variables|wall_inside|Getwall__inside_con_count) (Variables|Wall|Getwall_length)) _wall_con_width _wall_con_width) 0.0) "0,90.000000, 0" "1,1,1"))
      (else
        (Variables|wall_inside|SetinsideDoor_count (Math|Integer|Clamp(Integer) (Variables|wall_inside|GetinsideDoor_count) 1 (Variables|Wall|GetY_wall_count)))
        (AddComponent|AddChildActorComponent false (Math|Transform|MakeTransform (Math|Vector|MakeVector (+ (* (+ (Variables|wall_inside|Getwall__inside_con_count) 1) (Variables|Wall|Getwall_length)) (Variables|Conner|Getwall_con_width)) (+ (Variables|Conner|Getwall_con_length) (* (Variables|wall_inside|GetinsideDoor_count) (Variables|Wall|Getwall_length))) 0.0) "0, 0, 0" "1,1,1"))))
    (else
      ;[1 1 1] 放置 外门
      (if (Variables|Door|Getdoor_is_inY?)
        (Variables|Door|Setdoor_in_count (Math|Integer|Clamp(Integer) (Variables|Door|Getdoor_in_count) 0 (- (Variables|Wall|GetY_wall_count) 1)))
        (AddComponent|AddChildActorComponent false (Math|Transform|MakeTransform (Math|Vector|MakeVector (Variables|Conner|Getwall_con_width) (+ (* (Math|Integer|Clamp(Integer) (Variables|Door|Getdoor_in_count) 0 (- (Variables|Wall|GetY_wall_count) 1)) (Variables|Wall|Getwall_length)) (Variables|Conner|Getwall_con_length)) 0.0) "0,-180.000000, 0" "1,1,1"))
        (else
          (Variables|Door|Setdoor_in_count (Math|Integer|Clamp(Integer) (Variables|Door|Getdoor_in_count) 0 (- (Variables|Wall|GetX_wall_count) 1)))
          (AddComponent|AddChildActorComponent false (Math|Transform|MakeTransform (Math|Vector|MakeVector (+ (* (Math|Integer|Clamp(Integer) (Variables|Door|Getdoor_in_count) 0 (- (Variables|Wall|GetX_wall_count) 1)) (Variables|Wall|Getwall_length)) (Variables|Conner|Getwall_con_length)) 0.0 0.0) "0,90.000000, 0" "1,1,1")))))))

(fn FUCSetInsideWall
  (bind _x_wall_count (Variables|Wall|GetX_wall_count))
  (bind _y_wall_count (Variables|Wall|GetY_wall_count))
  ;[1 1 1] 生成内墙
  (if (Variables|wall_inside|Gethas_Inside_Wall?)
    (if (Variables|wall_inside|GetinsideWall_is_inY?)
      (bind _output_get (Variables|wall_inside|Setwall__inside_con_count (Math|Integer|Clamp(Integer) (Variables|wall_inside|Getwall__inside_con_count) 0 (- (Variables|Wall|GetY_wall_count) 1))))
      (if (Variables|Door|Getdoor_is_inY?)
        (if (== _output_get (Variables|Door|Getdoor_in_count))
          (Variables|wall_inside|Sethas_Inside_Wall? false)
          (else
            (AddComponent|AddStaticMeshComponent false (Math|Transform|MakeTransform (Math|Vector|MakeVector 0.0 (+ (Variables|Conner|Getwall_con_length) (* (Variables|wall_inside|Getwall__inside_con_count) (Variables|Wall|Getwall_length))) 0.0) "0, 0, 0" "1,1,1") :!label _label)
            (AddComponent|AddStaticMeshComponent false (Math|Transform|MakeTransform (Math|Vector|MakeVector (+ (* (Variables|Wall|GetX_wall_count) (Variables|Wall|Getwall_length)) (Variables|Conner|Getwall_con_length) (Variables|Conner|Getwall_con_length)) (+ (Variables|Conner|Getwall_con_length) (* (Variables|wall_inside|Getwall__inside_con_count) (Variables|Wall|Getwall_length))) 0.0) "0, 0, 0" "-1.000000,1,1"))
            (CallFunction|FUCSetDoor true :!label _label_2)
            (if (Variables|wall_inside|GetinsideWall_is_inY?)
              (if (> _x_wall_count 1)
                (for _index (range 0 (- _x_wall_count 1))
                  (if (not (== _index (Variables|wall_inside|GetinsideDoor_count)))
                    (AddComponent|AddChildActorComponent false (Math|Transform|MakeTransform (Math|Vector|MakeVector (+ (* _index (Variables|Wall|Getwall_length)) (Variables|Conner|Getwall_con_length)) (+ (* (Variables|wall_inside|Getwall__inside_con_count) (Variables|Wall|Getwall_length)) (Variables|Conner|Getwall_con_length)) 0.0) "0, 0, 0" "1,1,1")))))
              (elif (> _y_wall_count 1)
                (for _index_2 (range 0 (- _y_wall_count 1))
                  (if (not (== (+ _index_2 1) (Variables|wall_inside|GetinsideDoor_count)))
                    (AddComponent|AddChildActorComponent false (Math|Transform|MakeTransform (Math|Vector|MakeVector (+ (* (Variables|wall_inside|Getwall__inside_con_count) (Variables|Wall|Getwall_length)) (Variables|Conner|Getwall_con_length) (Variables|wall_inside|Getinside_wall_length)) (+ (* _index_2 (Variables|Wall|Getwall_length)) (Variables|Conner|Getwall_con_length)) 0.0) "0,90.000000, 0" "1,1,1"))))))))
        (else
          (goto _label)))
      (else
        (bind _output_get_2 (Variables|wall_inside|Setwall__inside_con_count (Math|Integer|Clamp(Integer) (Variables|wall_inside|Getwall__inside_con_count) 0 (- (Variables|Wall|GetX_wall_count) 1))))
        (if (Variables|Door|Getdoor_is_inY?)
          (AddComponent|AddStaticMeshComponent false (Math|Transform|MakeTransform (Math|Vector|MakeVector (+ (* (Variables|wall_inside|Getwall__inside_con_count) (Variables|Wall|Getwall_length)) (Variables|Conner|Getwall_con_length) (Variables|wall_inside|Getinside_wall_length)) 0.0 0.0) "0,90.000000, 0" "1,1,1") :!label _label_3)
          (AddComponent|AddStaticMeshComponent false (Math|Transform|MakeTransform (Math|Vector|MakeVector (+ (* (Variables|wall_inside|Getwall__inside_con_count) (Variables|Wall|Getwall_length)) (Variables|Conner|Getwall_con_length) (Variables|wall_inside|Getinside_wall_length)) (+ (* (Variables|Wall|GetY_wall_count) (Variables|Wall|Getwall_length)) (Variables|Conner|Getwall_con_length) (Variables|Conner|Getwall_con_length)) 0.0) "0,90.000000, 0" "-1.000000,1,1"))
          (goto _label_2)
          (elif (== _output_get_2 (Variables|Door|Getdoor_in_count))
            (Variables|wall_inside|Sethas_Inside_Wall? false)
            (else
              (goto _label_3))))))))