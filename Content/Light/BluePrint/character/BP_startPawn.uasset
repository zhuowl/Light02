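; BP_startPawn is the start pawn, which shows the start menu when play begins.
; BeginPlay enables the mouse cursor, then creates the UMG_start widget and adds it to the viewport.
; The turn axis events are empty; disconnected leftover nodes hold clamped yaw look, rate-based turning and an arrow-direction line trace for BP_character_girl, none of which run.
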(event EventBeginPlay
  (Variables|/Script/Engine.PlayerController|SetbShowMouseCursor (Game|GetPlayerController 0) true)
  (bind _returnvalue (UserInterface|CreateWidget "/Game/Light/UI/UMG_start.UMG_start_C"))
  (UserInterface|Viewport|AddtoViewport _returnvalue 0))

(event Collision|EventActorBeginOverlap
  (params (OtherActor :type Actor%20Object%20Reference)))

(event EventTick
  (params (DeltaSeconds :type Float%20%28single-precision%29)))

(event Input|AxisEvents|InputAxisTurnRate
  (params (AxisValue :type Float%20%28single-precision%29))
  ;[1 1 1] Gamepad_input
)

(event Input|AxisEvents|InputAxisTurn
  (params (AxisValue :type Float%20%28single-precision%29))
  ;[1 1 1] Mouse_input
)

(fn ConstructionScript)