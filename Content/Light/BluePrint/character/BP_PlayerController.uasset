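; BP_PlayerController is a player controller that toggles the game's pause menu with the Enter key.
; A FlipFlop alternates between pausing and unpausing, feeding its state straight into SetGamePaused.
; Pausing creates a new UMG_pause widget and adds it to the viewport, while unpausing removes it.
; Both branches set the mouse cursor visible, so it stays shown after resuming.
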(event EventBeginPlay)

(event EventTick
  (params (DeltaSeconds :type Float%20%28single-precision%29)))

(event Input|KeyboardEvents|Enter
  (params (Key :type Key%20Structure))
  (:Pressed
    (bind _isa (Utilities|FlowControl|FlipFlop)
      (:A
        (Game|SetGamePaused _isa)
        (bind _returnvalue (UserInterface|CreateWidget "/Game/Light/UI/UMG_pause.UMG_pause_C"))
        (bind _output_get (Variables|Default|SetUI_pause _returnvalue))
        (UserInterface|Viewport|AddtoViewport _output_get 0)
        (Variables|/Script/Engine.PlayerController|SetbShowMouseCursor self true))
      (:B
        (Game|SetGamePaused _isa)
        (Widget|RemovefromParent (Variables|Default|GetUI_pause))
        (Variables|/Script/Engine.PlayerController|SetbShowMouseCursor self true)))))

(fn ConstructionScript)