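; Samurai enemy AI that patrols, hunts the player's girl character and reports a lost game to BP_manager on reaching her.
; PawnSensing sight starts a chase, with a retriggerable delay clearing it when sightings stop, while her noises send it to investigate.
; Self-re-calling AIMoveTo events drive patrol, hearing and chase at different speeds, without a behavior tree.
; A box overlap randomly opens closed doors immediately or re-routes patrol first.
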(event OnSeePawn(PawnSensing)
  (params (Pawn :type Pawn%20Object%20Reference))
  ;[1 1 1] see_player
  (bind _asbp_character_girl (Utilities|Casting|CastToBP_character_girl Pawn))
  (Variables|Default|Setplayer _asbp_character_girl)
  (Variables|Default|SetSeePlayer? true)
  (Utilities|FlowControl|Sequence
    (:then_0
      (Utilities|FlowControl|DoOnce false
        (:Completed
          (CallFunction|FollowPlayer))))
    (:then_1
      (Utilities|FlowControl|RetriggerableDelay 0.6)
      (Variables|Default|SetSeePlayer? false)
      (CallFunction|ResetFollow))))

(event OnHearNoise(PawnSensing)
  (params (Instigator :type Pawn%20Object%20Reference) (Location :type Vector%20%28by%20ref%29 :default "0, 0, 0") (Volume :type Float%20%28single-precision%29))
  (bind _bsuccess (Utilities|Casting|CastToBP_character_girl Instigator))
  ;[1 1 1] hear_sound
  (Variables|Default|Setis_hearig? _bsuccess)
  (if _bsuccess
    (Variables|Default|Setnoise_location Location)
    (CallFunction|Hearing)))

(event OnComponentBeginOverlap(Box)
  (params (OverlappedComponent :type Primitive%20Component%20Object%20Reference) (OtherActor :type Actor%20Object%20Reference) (OtherComp :type Primitive%20Component%20Object%20Reference) (OtherBodyIndex :type Integer) (bFromSweep :type Boolean) (SweepResult :type Hit%20Result%20Structure%20%28by%20ref%29))
  ;[1 1 1] open_door
  (bind _asbp_door (Utilities|Casting|CastToBP_door OtherActor))
  (Variables|Default|Setdoor _asbp_door)
  (if (not (Variables|/Game/Light/BluePrint/common/BP_door.BP_door_C|Getopen? (Variables|Default|Getdoor)))
    (if (> (Math|Random|RandomFloatinRange 0.0 1.0) (Variables|Default|GetopenDoor))
      (if (Variables|Default|GetisPatrol)
        (Math|Integer|IncrementInt (Variables|Default|GetTraget_count)
          (:%20%20
            _)))
      (CallFunction|Patrol)
      (Utilities|FlowControl|Delay 1.0)
      (if (Collision|IsOverlappingActor (Variables|Default|GetBox) (Variables|Default|Getdoor) :!class /Script/Engine.PrimitiveComponent)
        (Default|DoorOpen (Variables|Default|Getdoor) self))
      (else
        (Default|DoorOpen (Variables|Default|Getdoor) self)))))

(event Custom|follow_player
  ;[1 1 1] follow
  (if (Variables|Default|GetSeePlayer?)
    (Variables|/Script/Engine.CharacterMovementComponent|SetMaxWalkSpeed (Variables|Character|GetCharacterMovement) 4.5e+02)
    (AI|AIMoveTo self "0, 0, 0" (Variables|Default|Getplayer) 1e+01 false
      (:then
        (Utilities|FlowControl|Delay 0.5)
        (if (Variables|Default|GetSeePlayer?)
          (CallFunction|FollowPlayer)
          (else
            (CallFunction|Patrol :!label _label)
            (CallFunction|ResetFollow))))
      (:OnSuccess
        (Utilities|FlowControl|DoOnce false
          (:Completed
            (Default|GameOver (Variables|Default|Getmanger) false))))
      (:OnFail
        (goto _label)))))

(event Custom|hearing
  ;[1 1 1] hearing
  (if (Variables|Default|GetSeePlayer?)
    (CallFunction|FollowPlayer)
    (else
      (Variables|/Script/Engine.CharacterMovementComponent|SetMaxWalkSpeed (Variables|Character|GetCharacterMovement) 6e+02)
      (AI|AIMoveTo self (Variables|Default|Getnoise_location) 0 5.0 false
        (:then
          (if (Variables|Default|GetSeePlayer?)
            (CallFunction|FollowPlayer)))
        (:OnSuccess
          (if (Variables|Default|GetSeePlayer?) :!label _label
            (CallFunction|FollowPlayer)
            (else
              (Utilities|FlowControl|Delay 0.2)
              (CallFunction|Patrol))))
        (:OnFail
          (goto _label))))))

(event Custom|Patrol
  (bind _patrol_point (Variables|Default|Getpatrol_point))
  ;[1 1 1] 巡逻
  (if (Variables|Default|GetSeePlayer?)
    (CallFunction|FollowPlayer)
    (else
      (Variables|Default|SetisPatrol true)
      (if (> (Variables|Default|GetTraget_count) (- (Utilities|Array|Length _patrol_point) 1))
        (Variables|Default|SetTraget_count 0))
      (Variables|Default|Settarget (Utilities|Array|Get(acopy) _patrol_point (Variables|Default|GetTraget_count)))
      (Variables|/Script/Engine.CharacterMovementComponent|SetMaxWalkSpeed (Variables|Character|GetCharacterMovement) 3e+02)
      (AI|AIMoveTo self "0, 0, 0" (Variables|Default|Gettarget) 1e+01 false
        (:OnSuccess
          _)
        (:OnFail
          _))
      (Variables|Default|SetTraget_count (+ (Variables|Default|GetTraget_count) 1))
      (CallFunction|Patrol))))

(event Custom|reset_follow
  ;[1 1 1] see_player
  (Utilities|FlowControl|DoOnce false) ; enters at Reset
)

(event EventBeginPlay
  (bind _outactors (Actor|GetAllActorsOfClass "/Game/Light/BluePrint/Game/BP_manager.BP_manager_C"))
  (Variables|Default|Setmanger (Utilities|Array|Get(acopy) _outactors))
  (Variables|Default|Settarget (Utilities|Array|Get(acopy) (Variables|Default|Getpatrol_point)))
  (CallFunction|Patrol))

(event Collision|EventActorBeginOverlap
  (params (OtherActor :type Actor%20Object%20Reference)))

(event EventTick
  (params (DeltaSeconds :type Float%20%28single-precision%29))
  (if (Variables|Default|GetSeePlayer?)
    _))

(fn ConstructionScript)